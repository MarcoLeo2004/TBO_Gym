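; BP_Patrol is a patrol route that supplies world-space waypoints from the points of its PatrolSpline.
; GetSplinePoint returns the location of the spline point at the current PointIndex.
; IncrementPoint steps the index by Direction and flips Direction at the last and first points, so the route runs back and forth rather than looping.
; It moves nothing itself and only tracks the current point.
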(event `IncrementPoint`
  (bind _output_get (set `self.PointIndex` (+ (`self.PointIndex`) (`self.Direction`))))
  (if (== _output_get (- (`SplineComponent.GetNumberOfSplinePoints` (`self.PatrolSpline`)) 1))
    (set `self.Direction` -1)
    (elif (== (`self.PointIndex`) 0)
      (set `self.Direction` 1))))

(fn `GetSplinePoint`
  (returns (PointPosition :type "Vector Structure"))
  (return (`SplineComponent.GetLocationAtSplinePoint` (`self.PatrolSpline`) (`self.PointIndex`) "World")))

(fn `UserConstructionScript`)