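; Enemy AI controller that starts the BHT_Enemy behavior tree on possessing a pawn.
; Three setter functions switch the AI state between idle, patrolling and attacking.
; Each stores the state in AIStates and writes it as an enum to the Blackboard key named by PlayerKeyName.
; The controller's own graphs never call these setters.
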(event `self.ReceivePossess`
  (params (PossessedPawn :type "Pawn Object Reference"))
  (`self.RunBehaviorTree` "/Game/Enemy/BHT_Enemy.BHT_Enemy"))

(fn `SetStateAsAttacking`
  (bind _output_get (set `self.AIStates` "NewEnumerator2"))
  (`BlackboardComponent.SetValueAsEnum` (`self.Blackboard`) (`self.PlayerKeyName`) _output_get))

(fn `SetStateAsIdle`
  (bind _output_get (set `self.AIStates` "NewEnumerator0"))
  (`BlackboardComponent.SetValueAsEnum` (`self.Blackboard`) (`self.PlayerKeyName`) _output_get))

(fn `SetStateAsPatrolling`
  (bind _output_get (set `self.AIStates` "NewEnumerator1"))
  (`BlackboardComponent.SetValueAsEnum` (`self.Blackboard`) (`self.PlayerKeyName`) _output_get))

(fn `UserConstructionScript`)