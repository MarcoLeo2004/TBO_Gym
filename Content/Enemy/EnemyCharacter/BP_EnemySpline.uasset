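; BP_EnemySpline is an enemy character that exposes a patrol spline route and switches AI state when it spots a pawn.
; It starts in a default state, and the FieldOfView sight event sets a new state and changes walk speed.
; State changes write the enum and the player character to the Blackboard.
; Tick draws a debug cone along its forward vector.
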(event `self.ReceiveBeginPlay`
  (set `self.AIStates` "NewEnumerator1"))

(event `self.FieldOfView.OnSeePawn`
  (params (Pawn :type "Pawn Object Reference"))
  (`self.SetValueBlackboardEnum` "NewEnumerator3")
  (set `CharacterMovementComponent.MaxWalkSpeed` 400.0 (`self.CharacterMovement`)))

(event `self.ReceiveTick`
  (params (DeltaSeconds :type "Float (single-precision)"))
  (`KismetSystemLibrary.DrawDebugConeInDegrees` (`self.K2_GetActorLocation`) (`self.GetActorForwardVector`) 1500.0 30.0 30.0 12 (struct :`G` 0.395474 :`B` 0.633681 :`A` 1.0) 0.1))

(fn `GetPatrolRoute`
  (returns (PatrolRoute :type "/Game/Blueprints/Movement/BP_Patrol Object Reference"))
  (return (`self.PatrolSpline`)))

(fn `SetValueBlackboardEnum`
  (params (AIStates :type "/Game/Blueprints/AIStates Enum" :default "NewEnumerator1"))
  (bind _returnvalue (`AIBlueprintHelperLibrary.GetBlackboard` null))
  (bind _output_get (set `self.AIStates` AIStates))
  (`BlackboardComponent.SetValueAsEnum` _returnvalue (`self.StateKeyName`) _output_get)
  (`BlackboardComponent.SetValueAsObject` _returnvalue (`self.KeyName`) (`GameplayStatics.GetPlayerCharacter` 0)))

(fn `UserConstructionScript`)