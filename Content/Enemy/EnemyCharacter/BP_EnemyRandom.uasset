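; Enemy character that wanders the navmesh and sprints after pawns it sees.
; It chains random AI moves within a large radius around itself, starting at BeginPlay.
; Its FieldOfView sighting event starts a chase, with a DoOnce gating the walk speed boost.
; A retriggerable delay after the latest sighting lowers the speed, rearms the sprint and resumes wandering.
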(event `self.ReceiveBeginPlay`
  (`self.MoveToRandomLocation`))

(event `MoveToRandomLocation`
  (bind _randomlocation (`NavigationSystemV1.K2_GetRandomLocationInNavigableRadius` (`self.K2_GetActorLocation`) 4000.0 null null))
  (`|AIMoveTo` self _randomlocation null
    (:`OnSuccess`
      (`self.MoveToRandomLocation`))))

(event `CanSprintAgain`
  (goto _label :!via `Reset`))

(event `self.FieldOfView.OnSeePawn`
  (params (Pawn :type "Pawn Object Reference"))
  (`|ExecutionSequence`
    (:`then_0`
      (`/Engine/EditorBlueprintResources/StandardMacros.DoOnce` false :!label _label
        (:`Completed`
          (set `CharacterMovementComponent.MaxWalkSpeed` 650.0 (`self.CharacterMovement`)))))
    (:`then_1`
      (`|AIMoveTo` self (0.0 0.0 0.0) Pawn
        (:`then`
          (`KismetSystemLibrary.RetriggerableDelay` 2.0)
          (set `CharacterMovementComponent.MaxWalkSpeed` 400.0 (`self.CharacterMovement`))
          (`self.CanSprintAgain`)
          (`self.MoveToRandomLocation`))))))

(fn `UserConstructionScript`)