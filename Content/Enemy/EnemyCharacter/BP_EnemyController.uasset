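; AI controller for the enemy character that drives its behavior through a behavior tree.
; On possess, it runs BHT_Enemy.
; Two functions switch the enemy to patrolling or running by setting the AIStates enum and writing it to the Blackboard state key.
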(event `self.ReceivePossess`
  (params (PossessedPawn :type "Pawn Object Reference"))
  (`self.RunBehaviorTree` "/Game/Enemy/BehaviorTree/BHT_Enemy.BHT_Enemy"))

(fn `SetStateAsPatrolling`
  (bind _output_get (set `self.AIStates` "NewEnumerator1"))
  (`BlackboardComponent.SetValueAsEnum` (`self.Blackboard`) (`self.StateKeyName`) _output_get))

(fn `SetStateAsRunning`
  (bind _output_get (set `self.AIStates` "NewEnumerator3"))
  (`BlackboardComponent.SetValueAsEnum` (`self.Blackboard`) (`self.StateKeyName`) _output_get))

(fn `UserConstructionScript`)